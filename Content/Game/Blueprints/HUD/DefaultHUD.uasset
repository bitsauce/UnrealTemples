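; DefaultHUD is a HUD Blueprint that draws a single text message on screen, chosen by priority level.
; SetMessage stores text in the Messages array at its level, growing the array as needed.
; DrawHUD scans from the highest level down for the first non-empty entry and draws it horizontally centered at a fixed height, using the measured text width.
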(event `self.ReceiveDrawHUD`
  (params (SizeX :type Integer) (SizeY :type Integer))
  (bind _messages (`self.Messages`))
  (bind _returnvalue (`KismetArrayLibrary.Array_Length` _messages))
  (for _index (range (+ _returnvalue 1))
    (bind _returnvalue_2 (- (- _returnvalue 1) _index))
    (if (`KismetStringLibrary.NotEqual_StrStr` (`KismetArrayLibrary.Array_Get` _messages _returnvalue_2))
      (break)))
  (bind _item (`KismetArrayLibrary.Array_Get` _messages _returnvalue_2))
  (`self.DrawText` _item (struct :`A` 1) (- (`KismetMathLibrary.Conv_IntToDouble` (/ SizeX 2)) (/ (`self.GetTextSize` _item "/Game/Game/Blueprints/HUD/ScreenFont.ScreenFont") 2.0)) 400.0 "/Game/Game/Blueprints/HUD/ScreenFont.ScreenFont" 1.0))

(fn `SetMessage`
  (params (Message :type String) (Level :type Integer))
  (`KismetArrayLibrary.Array_Set` (`self.Messages`) Level Message true))

(fn `UserConstructionScript`)