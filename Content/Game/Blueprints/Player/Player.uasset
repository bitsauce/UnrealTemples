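; Player character Blueprint that spawns and attaches a sword and shield, and handles lock-on, interaction and ladder volumes.
; Lock-on toggles on the nearest in-range Enemy; Tick then faces it, sets strafe-aware MovementDirection and eases controller yaw with an angle-scaled correction.
; The nearest Interactable in range supplies the HUD prompt each tick and receives the Interact press.
; Ladder volume overlaps stop movement and switch gravity off until exit.
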(event `self.ReceiveBeginPlay`
  (`|ExecutionSequence`
    (:`then_0`
      (bind _returnvalue (`|SpawnActorFromClass` "/Game/Game/Blueprints/Weapons/Weapon_Sword.Weapon_Sword_C" (`KismetMathLibrary.MakeTransform` (0.0 0.0 0.0))))
      (`KismetArrayLibrary.Array_Add` (`/Game/Game/Blueprints/Weapons/Weapon_Sword.ActorsToIgnore` _returnvalue) self)
      (set `/Game/Game/Blueprints/Weapons/Weapon_Sword.Holder` self _returnvalue)
      (bind _output_get (set `self.EquipedR` _returnvalue))
      (`self.K2_AttachRootComponentTo` _output_get (`self.Mesh`) "hand_rSocket" "KeepRelativeOffset" true))
    (:`then_1`
      (bind _returnvalue_2 (`|SpawnActorFromClass` "/Game/Game/Blueprints/Weapons/Shield.Shield_C" (`KismetMathLibrary.MakeTransform` (0.0 0.0 0.0))))
      (`KismetArrayLibrary.Array_Add` (`/Game/Game/Blueprints/Weapons/Weapon_Sword.ActorsToIgnore` _returnvalue) _returnvalue_2)
      (bind _output_get_2 (set `self.EquipedL` _returnvalue_2))
      (`self.K2_AttachRootComponentTo` _output_get_2 (`self.Mesh`) "lowerarm_lSocket" "KeepRelativeOffset" true))))

(event `InputAction|Interact`
  ;[1 1 1] Use interactions
  (:`Pressed`
    (set `self.MinDistance` 10000000.0)
    (bind _outactors (`GameplayStatics.GetAllActorsWithInterface` "/Game/Game/Blueprints/Interactables/Interactable.Interactable_C"))
    (for _array_element _outactors
      (bind _returnvalue (`KismetMathLibrary.VSize` (- (`self.K2_GetActorLocation` _array_element) (`self.K2_GetActorLocation`))))
      (if (< _returnvalue (`self.MinDistance`))
        (set `self.ClosestActor` _array_element)
        (set `self.MinDistance` _returnvalue)))
    (if (< (`self.MinDistance`) (`self.MaxUseDistance`))
      (message `/Game/Game/Blueprints/Interactables/Interactable.OnInteract` (`self.ClosestActor`) self))))

(event `InputAction|LockOn`
  ;[1 1 1] Lock-on logic
  (:`Pressed`
    (`/Engine/EditorBlueprintResources/StandardMacros.IsValid` (`self.LockOnTarget`)
      (:`Is Valid`
        (set `self.LockOnTarget` null))
      (:`Is Not Valid`
        (set `self.MinDistance` 10000000.0)
        (bind _outactors (`GameplayStatics.GetAllActorsOfClass` "/Game/Game/Blueprints/Enemies/Enemy.Enemy_C"))
        (for _array_element _outactors
          (bind _returnvalue (`KismetMathLibrary.VSize` (- (`self.K2_GetActorLocation` _array_element) (`self.K2_GetActorLocation`))))
          (if (< _returnvalue (`self.MinDistance`))
            (set `self.ClosestActor` _array_element)
            (set `self.MinDistance` _returnvalue)))
        (if (< (`self.MinDistance`) (`self.MaxLockOnDistance`))
          (set `self.LockOnTarget` (`self.ClosestActor`)))))))

(event `self.ReceiveActorBeginOverlap`
  (params (OtherActor :type "Actor Object Reference"))
  ;[1 1 1] Ladder logic
  (cast `/Game/Game/Blueprints/Interactables/LadderVolume` OtherActor)
  (set `CharacterMovementComponent.GravityScale` 0.0 (`self.CharacterMovement`))
  (`MovementComponent.StopMovementImmediately`))

(event `self.ReceiveActorEndOverlap`
  (params (OtherActor :type "Actor Object Reference"))
  ;[1 1 1] Ladder logic
  (cast `/Game/Game/Blueprints/Interactables/LadderVolume` OtherActor)
  (set `CharacterMovementComponent.GravityScale` 1.0 (`self.CharacterMovement`)))

(event `self.ReceiveTick`
  (params (DeltaSeconds :type "Float (single-precision)"))
  (bind _returnvalue (`KismetMathLibrary.MakeVector2D` (`self.GetInputAxisValue`) (`self.GetInputAxisValue`)))
  (`parent.ReceiveTick` DeltaSeconds)
  (`|ExecutionSequence`
    (:`then_0`
      (`/Engine/EditorBlueprintResources/StandardMacros.IsValid` (`self.LockOnTarget`)
        (:`Is Valid`
          (set `self.MovementDirection` _returnvalue)
          (`self.SetActorRotation` (`KismetMathLibrary.ComposeRotators` (`KismetMathLibrary.MakeRotFromX` (`KismetMathLibrary.Normal` (`KismetMathLibrary.MakeVector` (.x (- (`self.K2_GetActorLocation`) (`self.K2_GetActorLocation` (`self.LockOnTarget`)))) (.y (- (`self.K2_GetActorLocation`) (`self.K2_GetActorLocation` (`self.LockOnTarget`))))))) (struct :`Yaw` 180.0)))
          (bind _transitionrotation (`self.CheckForRotationToLock`)
            (:`UpdateNeeded`
              (`self.AddControllerYawInput` _transitionrotation))))
        (:`Is Not Valid`
          (set `self.MovementDirection` (`KismetMathLibrary.MakeVector2D` 0.0 (`KismetMathLibrary.VSize2D` _returnvalue))))))
    (:`then_1`
      (set `self.MinDistance` 10000000.0)
      (bind _outactors (`GameplayStatics.GetAllActorsWithInterface` "/Game/Game/Blueprints/Interactables/Interactable.Interactable_C"))
      (for _array_element _outactors
        (bind _returnvalue_2 (`KismetMathLibrary.VSize` (- (`self.K2_GetActorLocation` _array_element) (`self.K2_GetActorLocation`))))
        (if (< _returnvalue_2 (`self.MinDistance`))
          (set `self.ClosestActor` _array_element)
          (set `self.MinDistance` _returnvalue_2)))
      (bind _returnvalue_3 (`Controller.CastToPlayerController` (`self.GetController`)))
      (bind _asdefault_hud (cast `/Game/Game/Blueprints/HUD/DefaultHUD` (`PlayerController.GetHUD` _returnvalue_3)))
      (if (< (`self.MinDistance`) (`self.MaxUseDistance`))
        (bind _asinteractable (cast `/Game/Game/Blueprints/Interactables/Interactable` (`self.ClosestActor`)))
        (bind _interactstring (`/Game/Game/Blueprints/Interactables/Interactable.GetInteractString` _asinteractable))
        (`/Game/Game/Blueprints/HUD/DefaultHUD.SetMessage` _asdefault_hud _interactstring 0)
        (else
          (`/Game/Game/Blueprints/HUD/DefaultHUD.SetMessage` _asdefault_hud "" 0))))))

(fn `UserConstructionScript`)