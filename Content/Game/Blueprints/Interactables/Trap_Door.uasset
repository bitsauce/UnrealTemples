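; Interactable trap door that swings open when interacted with.
; OnInteract plays the Open timeline from the start, whose Angle track sets the relative pitch in two opposite directions, negated and positive.
; An Opening flag ignores further interactions until the timeline finishes.
; GetInteractString returns an empty string.
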(event `/Game/Game/Blueprints/Interactables/Interactable.OnInteract`
  (params (Player :type "/Game/Game/Blueprints/Player/Player Object Reference"))
  (if (not (`self.Opening`))
    (set `self.Opening` true)
    (bind (_direction _angle) (`Timeline|Open` :!via `PlayFromStart`)
      (:`Update`
        (`SceneComponent.K2_SetRelativeRotation` (`KismetMathLibrary.MakeRot` (* _angle -1.0)))
        (`SceneComponent.K2_SetRelativeRotation` (`KismetMathLibrary.MakeRot` _angle)))
      (:`Finished`
        (set `self.Opening` false)))))

(fn `GetInteractString`
  (returns (InteractString :type String))
  (return ""))

(fn `UserConstructionScript`)