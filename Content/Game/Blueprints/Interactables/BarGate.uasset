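; BarGate is an interactable hinged gate that players can open, close and unlock with a key, with separate front and back locks.
; A dot product against the gate's right vector picks which lock applies and which of two timelines swings it in opposite yaw directions.
; A matching inventory key clears both locks, while fully opening from an unlocked side clears the opposite one.
; OpenState and FlipFlops route later interactions to reverse the active swing.
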(event `/Game/Game/Blueprints/Interactables/Interactable.OnInteract`
  (params (Player :type "/Game/Game/Blueprints/Player/Player Object Reference"))
  (if (== (`self.OpenState`) 0)
    (if (< (`KismetMathLibrary.Dot_VectorVector` (- (`self.K2_GetActorLocation` Player) (`self.K2_GetActorLocation`)) (`SceneComponent.GetRightVector`)) 0.0)
      (if (`self.LockedFront`)
        (for _array_element (`/Game/Game/Blueprints/Player/Player.Inventory` Player) :!label _label
          (if (`KismetStringLibrary.EqualEqual_StrStr` _array_element (`self.KeyName`))
            (set `self.LockedBack` false)
            (set `self.LockedFront` false)
            (`KismetSystemLibrary.PrintString` "Door unlocked")))
        (if (or (`self.LockedFront`) (`self.LockedBack`))
          (`KismetSystemLibrary.PrintString` "Door locked"))
        (else
          (bind _isa (`/Engine/EditorBlueprintResources/StandardMacros.FlipFlop` :!label _label_2)
            (:`A`
              (bind (_direction _rotation) (`Timeline|OpenForwards` :!label _label_3)
                (:`Update`
                  (`SceneComponent.K2_SetRelativeRotation` (`KismetMathLibrary.MakeRot` 0.0 (* _rotation 90.0))))
                (:`Finished`
                  (if _isa
                    (set `self.OpenState` 1)
                    (set `self.LockedBack` false)
                    (else
                      (set `self.OpenState` 0))))))
            (:`B`
              (goto _label_3 :!via `Reverse`)))))
      (elif (`self.LockedBack`)
        (goto _label)
        (else
          (bind _isa_2 (`/Engine/EditorBlueprintResources/StandardMacros.FlipFlop` :!label _label_4)
            (:`A`
              (bind (_direction_2 _rotation_2) (`Timeline|OpenBack` :!label _label_5)
                (:`Update`
                  (`SceneComponent.K2_SetRelativeRotation` (`KismetMathLibrary.MakeRot` 0.0 (* _rotation_2 -90.0))))
                (:`Finished`
                  (if _isa_2
                    (set `self.OpenState` 2)
                    (set `self.LockedFront` false)
                    (else
                      (set `self.OpenState` 0))))))
            (:`B`
              (goto _label_5 :!via `Reverse`))))))
    (elif (== (`self.OpenState`) 1)
      (goto _label_2)
      (else
        (goto _label_4)))))

(fn `GetInteractString`
  (returns (InteractString :type String))
  (return "Press A to open door"))

(fn `UserConstructionScript`)