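; Sword weapon that kills characters on contact while its damage is enabled.
; Overlaps count only for actors outside the ignore list and while the holder's attack is not blocked.
; Hitting a Shield sets the holder's AttackBlocked flag for a brief delay, suppressing further hits.
; Any other CharacterMaster it touches is destroyed outright, with no damage calculation.
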(event `self.ReceiveActorBeginOverlap`
  (params (OtherActor :type "Actor Object Reference"))
  (bind _holder (`self.Holder`))
  (if (`KismetArrayLibrary.Array_Contains` (`self.ActorsToIgnore`) OtherActor)
    _
    (elif (and (`self.EnableDamage`) (not (`/Game/Game/Blueprints/CharacterMaster/CharacterMaster.AttackBlocked` (`self.Holder`))))
      (cast `/Game/Game/Blueprints/Weapons/Shield` OtherActor
        (:`then`
          (set `/Game/Game/Blueprints/CharacterMaster/CharacterMaster.AttackBlocked` true _holder)
          (`KismetSystemLibrary.Delay` 0.1)
          (set `/Game/Game/Blueprints/CharacterMaster/CharacterMaster.AttackBlocked` false _holder))
        (:`CastFailed`
          (bind _ascharacter_master (cast `/Game/Game/Blueprints/CharacterMaster/CharacterMaster` OtherActor))
          (`self.K2_DestroyActor` _ascharacter_master))))))

(fn `UserConstructionScript`)