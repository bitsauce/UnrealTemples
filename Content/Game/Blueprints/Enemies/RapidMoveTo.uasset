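; Behavior tree task that moves an enemy pawn toward its blackboard target, TargetToFollow.
; On execute it caches the BasicAIController, then runs AIMoveTo to a standoff point a fixed distance from the target, on the pawn's side.
; Only a successful move finishes the task, as failure is unhandled.
; A Tick event sets the EnableStrafe key according to whether the pawn is within close range of the target.
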(event `self.ReceiveExecute`
  (params (OwnerActor :type "Actor Object Reference"))
  (bind _returnvalue (`Controller.K2_GetPawn` (`self.AIController`)))
  (bind _returnvalue_2 (`Actor.K2_GetActorLocation` (`BTFunctionLibrary.GetBlackboardValueAsActor` (`self.TargetToFollow`))))
  (if (not (!= (`self.AIController`) null))
    (bind _asbasic_aicontroller (cast `/Game/Game/Blueprints/Enemies/BasicAIController` OwnerActor))
    (set `self.AIController` _asbasic_aicontroller))
  (`|AIMoveTo` _returnvalue (+ (* (`KismetMathLibrary.Normal` (- (`Actor.K2_GetActorLocation` _returnvalue) _returnvalue_2)) 250.0) _returnvalue_2) null 50.0
    (:`OnSuccess`
      (`self.FinishExecute` true))))

(event `self.ReceiveTick`
  (params (OwnerActor :type "Actor Object Reference") (DeltaSeconds :type "Float (single-precision)"))
  (`BTFunctionLibrary.SetBlackboardValueAsBool` (`self.EnableStrafe`) (<= (`KismetMathLibrary.VSize` (- (`Actor.K2_GetActorLocation` (`Controller.K2_GetPawn` (`self.AIController`))) (`Actor.K2_GetActorLocation` (`BTFunctionLibrary.GetBlackboardValueAsActor` (`self.TargetToFollow`))))) 300.0)))