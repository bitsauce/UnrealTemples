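; SwordFighter is an AI-controlled enemy that spawns a sword and shield on its hand and forearm sockets, with the sword ignoring both wielder and shield.
; Tick reads the blackboard: in strafe mode it either pulses Attacking or faces the target, setting MovementDirection to circle while holding a set distance.
; Otherwise it follows the AI controller's path, turning toward movement input at a capped rate through a wrapped-angle macro.
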(event `self.ReceiveBeginPlay`
  (`|ExecutionSequence`
    (:`then_0`
      (bind _returnvalue (`|SpawnActorFromClass` "/Game/Game/Blueprints/Weapons/Weapon_Sword.Weapon_Sword_C" (`KismetMathLibrary.MakeTransform` (0.0 0.0 0.0)) "AdjustIfPossibleButDontSpawnIfColliding" "OverrideRootScale"))
      (`KismetArrayLibrary.Array_Add` (`/Game/Game/Blueprints/Weapons/Weapon_Sword.ActorsToIgnore` _returnvalue) self)
      (set `/Game/Game/Blueprints/Weapons/Weapon_Sword.Holder` self _returnvalue)
      (bind _output_get (set `self.EquipedR` _returnvalue))
      (`self.K2_AttachRootComponentTo` _output_get (`self.Mesh`) "hand_rSocket" "KeepRelativeOffset" true))
    (:`then_1`
      (bind _returnvalue_2 (`|SpawnActorFromClass` "/Game/Game/Blueprints/Weapons/Shield.Shield_C" (`KismetMathLibrary.MakeTransform` (0.0 0.0 0.0)) "AdjustIfPossibleButDontSpawnIfColliding" "OverrideRootScale"))
      (`KismetArrayLibrary.Array_Add` (`/Game/Game/Blueprints/Weapons/Weapon_Sword.ActorsToIgnore` _returnvalue) _returnvalue_2)
      (bind _output_get_2 (set `self.EquipedL` _returnvalue_2))
      (`self.K2_AttachRootComponentTo` _output_get_2 (`self.Mesh`) "lowerarm_lSocket" "KeepRelativeOffset" true))))

(event `self.ReceiveTick`
  (params (DeltaSeconds :type "Float (single-precision)"))
  (bind _characterturnrate (`self.CharacterTurnRate`))
  (if (`BlackboardComponent.GetValueAsBool` (`AIBlueprintHelperLibrary.GetBlackboard` null) "EnableStrafe")
    (if (`BlackboardComponent.GetValueAsBool` (`AIBlueprintHelperLibrary.GetBlackboard` null) "EnableAttack")
      (set `self.Attacking` true)
      (`BlackboardComponent.SetValueAsBool` (`AIBlueprintHelperLibrary.GetBlackboard` null) "EnableAttack" false)
      (`KismetSystemLibrary.Delay` 0.1)
      (set `self.Attacking` false)
      (else
        (bind _asactor (cast `Actor` (`BlackboardComponent.GetValueAsObject` (`AIBlueprintHelperLibrary.GetBlackboard` null) "TargetToFollow")))
        (bind _returnvalue (- (`self.K2_GetActorLocation`) (`self.K2_GetActorLocation` _asactor)))
        (`self.SetActorRotation` (`KismetMathLibrary.ComposeRotators` (`KismetMathLibrary.MakeRotFromX` (`KismetMathLibrary.Normal` (`KismetMathLibrary.MakeVector` (.x _returnvalue) (.y _returnvalue)))) (struct :`Yaw` 180.0)))
        (set `self.MovementDirection` (`KismetMathLibrary.MakeVector2D` (`KismetMathLibrary.Conv_IntToDouble` (`BlackboardComponent.GetValueAsInt` (`AIBlueprintHelperLibrary.GetBlackboard` null) "StrafeDirection")) (`KismetMathLibrary.FClamp` (* (- (`KismetMathLibrary.VSize` _returnvalue) 250.0) 0.01) -1.0)))))
    (else
      (`SceneComponent.K2_AddWorldRotation` (`self.CapsuleComponent`) (`KismetMathLibrary.MakeRotator` 0.0 0.0 (* (`KismetMathLibrary.FClamp` (`self.NewMacro_0` (.yaw (`KismetMathLibrary.MakeRotFromX` (`KismetMathLibrary.GetForwardVector` (`SceneComponent.K2_GetComponentRotation` (`self.CapsuleComponent`))))) (.yaw (`KismetMathLibrary.MakeRotFromX` (`KismetMathLibrary.Normal` (`KismetMathLibrary.MakeVector` (.x (`self.GetLastMovementInputVector`)) (.y (`self.GetLastMovementInputVector`))))))) (* _characterturnrate -1.0) _characterturnrate) -1.0)) false false)
      (bind _returnvalue_2 (`AIBlueprintHelperLibrary.GetAIController` self))
      (if (`|EnumEquality` (`AIController.GetMoveStatus` _returnvalue_2) "Idle")
        (set `self.MovementDirection` (0.0 0.0))
        (else
          (`self.AddMovementInput` (`KismetMathLibrary.Normal` (- (`AIController.GetImmediateMoveDestination` _returnvalue_2) (`self.K2_GetActorLocation`))))
          (set `self.MovementDirection` (0.0 1.0)))))))

(fn `UserConstructionScript`)