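; Enemy behavior tree task that periodically flips the strafe direction stored on the Blackboard.
; On execute it sets the StrafeDirection key to positive one and starts a short randomized countdown.
; Tick decrements the timer, negates the key when it expires and rolls a new interval.
; The task only writes the direction, applying no movement itself and never calling Finish Execute.
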(event `self.ReceiveExecute`
  (params (OwnerActor :type "Actor Object Reference"))
  (`BTFunctionLibrary.SetBlackboardValueAsInt` (`self.StrafeDirection`) 1)
  (set `self.Timer` (`KismetMathLibrary.RandomFloatInRange` 1.0 3.0) :!label _label))

(event `self.ReceiveTick`
  (params (OwnerActor :type "Actor Object Reference") (DeltaSeconds :type "Float (single-precision)"))
  (bind _strafedirection (`self.StrafeDirection`))
  (bind _output_get (set `self.Timer` (- (`self.Timer`) DeltaSeconds)))
  (if (<= _output_get 0.0)
    (`BTFunctionLibrary.SetBlackboardValueAsInt` _strafedirection (* (`BTFunctionLibrary.GetBlackboardValueAsInt` _strafedirection) -1))
    (goto _label)))