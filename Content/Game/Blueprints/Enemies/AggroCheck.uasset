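; Behavior tree node that checks aggro for enemies, picking a target to follow on each tick.
; It sphere-traces around the pawn of its cached BasicAIController, ignoring all Enemy actors, then line-traces to each hit to confirm line of sight.
; The first visible actor sets the TargetToFollow and TargetLocation blackboard keys.
; Blocked hits clear only TargetToFollow, leaving the last known location, and an empty sweep changes neither key.
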(event `self.ReceiveTick`
  (params (OwnerActor :type "Actor Object Reference") (DeltaSeconds :type "Float (single-precision)"))
  (bind _returnvalue (`Actor.K2_GetActorLocation` (`Controller.K2_GetPawn` (`self.AIController`))))
  (if (not (!= (`self.AIController`) null))
    (bind _asbasic_aicontroller (cast `/Game/Game/Blueprints/Enemies/BasicAIController` OwnerActor))
    (set `self.AIController` _asbasic_aicontroller))
  (bind _outactors (`GameplayStatics.GetAllActorsOfClass` "/Game/Game/Blueprints/Enemies/Enemy.Enemy_C"))
  (set `self.MyLocation` _returnvalue)
  (bind _outhits (`KismetSystemLibrary.SphereTraceMultiForObjects` _returnvalue (+ _returnvalue (0.0 0.0 15.0)) 1500.0 (`self.DesiredObjectTypes`) false _outactors))
  (for _array_element _outhits
    (bind (_bblockinghit _binitialoverlap _time _location _impactpoint _normal _impactnormal _physmat _hitactor) (`GameplayStatics.BreakHitResult` _array_element))
    (bind _outhit (`KismetSystemLibrary.LineTraceSingleForObjects` (`self.MyLocation`) (`Actor.K2_GetActorLocation` _hitactor) (`|MakeArray` "ObjectTypeQuery1" "ObjectTypeQuery3" :!type "EObjectTypeQuery Enum") false _outactors))
    (bind (_bblockinghit_2 _binitialoverlap_2 _time_2 _location_2 _impactpoint_2 _normal_2 _impactnormal_2 _physmat_2 _hitactor_2) (`GameplayStatics.BreakHitResult` _outhit))
    (if (== _hitactor_2 _hitactor)
      (`BTFunctionLibrary.SetBlackboardValueAsObject` (`self.TargetToFollow`) _hitactor_2)
      (`BTFunctionLibrary.SetBlackboardValueAsVector` (`self.TargetLocation`) (`Actor.K2_GetActorLocation` _hitactor_2))
      (break)
      (else
        (`BTFunctionLibrary.SetBlackboardValueAsObject` (`self.TargetToFollow`))))))