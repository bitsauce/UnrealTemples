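; Interactable item pickup actor that adds its item to the interacting player's inventory.
; On interact, it looks up its ItemName row in ItemDataTable, prints a pickup message, adds the row to the player's Inventory and destroys itself.
; Nothing happens if the row is missing.
; GetInteractString supplies a fixed "Take item" button prompt.
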(event `/Game/Game/Blueprints/Interactables/Interactable.OnInteract`
  (params (Player :type "/Game/Game/Blueprints/Player/Player Object Reference"))
  (bind _returnvalue (`|GetDataTableRow` "/Game/Game/Blueprints/Items/ItemDataTable.ItemDataTable" (`KismetStringLibrary.Conv_StringToName` (`self.ItemName`)))
    (:`then`
      (`KismetSystemLibrary.PrintString` (`KismetStringLibrary.Concat_StrStr` (`.Name_4_C51A7EC84F5781FCA2883DB44F30C788` (break `/Game/Game/Blueprints/Items/ItemData` _returnvalue)) " picked up"))
      (`KismetArrayLibrary.Array_Add` (`/Game/Game/Blueprints/Player/Player.Inventory` Player) _returnvalue)
      (`self.K2_DestroyActor`))))

(fn `GetInteractString`
  (returns (InteractString :type String))
  (return "'A' Take item"))

(fn `UserConstructionScript`)